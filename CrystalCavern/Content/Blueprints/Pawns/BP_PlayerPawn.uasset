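; BP_PlayerPawn is a player pawn that moves by applying physics torque to its mesh.
; Forward/backward and left/right axis inputs apply torque around the world Y and X axes respectively, scaled by Acceleration.
; The torque is applied as an acceleration change, so the response is independent of mass.
; On BeginPlay, the player camera manager starts a camera fade from full opacity.
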(event `self.ReceiveBeginPlay`
  (`PlayerCameraManager.StartCameraFade` :`self` (`GameplayStatics.GetPlayerCameraManager` 0) :`FromAlpha` 1.0 :`Duration` 3.0))

(event `InputAxis|Move Forward/Backward`
  (params (AxisValue :type "Float (single-precision)"))
  (`PrimitiveComponent.AddTorqueInRadians` (`self.Mesh`) (`KismetMathLibrary.MakeVector` 0.0 (* AxisValue (`self.Acceleration`))) "None" true))

(event `InputAxis|Move Left/Right`
  (params (AxisValue :type "Float (single-precision)"))
  (`PrimitiveComponent.AddTorqueInRadians` (`self.Mesh`) (`KismetMathLibrary.MakeVector` (* AxisValue (`self.Acceleration`))) "None" true))

(fn `UserConstructionScript`)